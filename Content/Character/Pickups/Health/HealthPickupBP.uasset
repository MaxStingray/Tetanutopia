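; Health pickup Blueprint that drifts toward nearby PlayerRobot actors, acting like a magnet within a limited range.
; BeginPlay stores the spawn location, and Tick moves the pickup a small fraction of the way toward each robot overlapping PullInRadius.
; A squared-distance check against the spawn point leashes the movement, which is applied per frame without delta-time scaling or sweep.
; The graph contains no healing or collection logic.
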(event EventBeginPlay
  (Variables|Default|SetInitialPosition (Transformation|GetActorLocation)))

(event EventTick
  (params (DeltaSeconds :type Float%20%28single-precision%29))
  (bind _returnvalue (Transformation|GetActorLocation))
  (for _array_element (Collision|GetOverlappingActors (Variables|Default|GetPullInRadius) "/Script/GenTest.PlayerRobot" :!class /Script/Engine.PrimitiveComponent)
    (if (<= (Math|Vector|VectorLengthSquared (- (Variables|Default|GetInitialPosition) (+ _returnvalue (* (- (Transformation|GetActorLocation _array_element) _returnvalue) 0.025)))) 5e+05)
      (Transformation|SetActorLocation (+ _returnvalue (* (- (Transformation|GetActorLocation _array_element) _returnvalue) 0.025)) false false))))

(fn ConstructionScript)