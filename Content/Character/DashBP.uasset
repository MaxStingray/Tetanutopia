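; Dash Blueprint that relays dash start and end to the player character.
; DashStart plays a dash sound at player pawn 0's location, then casts that pawn to Player and calls its DashStart.
; Tick polls the Dashing flag and calls the Player's EndDashEvent on every frame it is false, rather than once when the dash ends.
; Nothing in this graph sets Dashing.
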(event EventBeginPlay)

(event EventTick
  (params (DeltaSeconds :type Float%20%28single-precision%29))
  (if (not (Variables|Default|GetbDashing))
    (bind _asplayer (Utilities|Casting|CastToPlayer (Game|Player|GetPlayerPawn 0)))
    (Default|EndDashEvent _asplayer)))

(event EventDashStart
  (Audio|PlaySoundatLocation "/Game/Audio/Sounds/Player_Dash1.Player_Dash1" (Transformation|GetActorLocation (Game|Player|GetPlayerPawn 0)))
  (bind _asplayer (Utilities|Casting|CastToPlayer (Game|Player|GetPlayerPawn 0)))
  (Default|DashStart _asplayer))