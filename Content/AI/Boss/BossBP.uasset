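; BossBP is a boss character Blueprint that arms itself with the OctoWeapon when play begins.
; After the parent BeginPlay, it equips the weapon, sets its projectile type to the slow projectile and offsets the spawn point forward along X.
; Overlap and Tick events are disabled stubs and the construction script only calls the parent, so any other behavior comes from the parent class.
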(event EventBeginPlay
  (bind _weapon (Variables|Default|Getweapon))
  (|CallParentFunction)
  (Class|BasicAI|EquipWeapon "/Game/Character/Weapons/TheOctoWeapon.TheOctoWeapon_C")
  (Variables|/Script/GenTest.BaseWeapon|SetProjectileType _weapon "/Game/Character/Projectiles/ProjectileSlow.ProjectileSlow_C")
  (Variables|/Script/GenTest.BaseWeapon|SetProjectileSpawnOffset _weapon "100.000000,0.000000, 0"))

(event Collision|EventActorBeginOverlap
  (params (OtherActor :type Actor%20Object%20Reference))
  (|CallParentFunction OtherActor) ; This node is disabled and will not be called.\nDrag off pins to build functionality.
)

(event EventTick
  (params (DeltaSeconds :type Float%20%28single-precision%29))
  (|CallParentFunction DeltaSeconds) ; This node is disabled and will not be called.\nDrag off pins to build functionality.
)

(fn ConstructionScript
  (|CallParentFunction))