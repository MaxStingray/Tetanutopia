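; Master AI enemy Blueprint that perceives the player robot and can drop health pickups on death.
; On BeginPlay it sets its weapon, health and speed from its controller.
; Perception updates for PlayerRobot write the CanSeePlayer flag to the Blackboard.
; OnDeath has a one-in-ten chance to spawn a health pickup, and it destroys the actor only within that same branch.
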(event OnTargetPerceptionUpdated(AIPerception)
  (params (Actor :type Actor%20Object%20Reference) (Stimulus :type AI%20Stimulus%20Structure))
  (Utilities|Casting|CastToPlayerRobot Actor)
  (if (.bSuccessfullySensed (Utilities|Struct|BreakAIStimulus Stimulus))
    (AI|Components|Blackboard|SetValueasBool (AI|GetBlackboard 0) (Variables|Default|GetCanSeePlayer) true)
    (else
      (AI|Components|Blackboard|SetValueasBool (AI|GetBlackboard 0) (Variables|Default|GetCanSeePlayer) false))))

(event EventBeginPlay
  (bind _self self)
  (CallFunction|SetWeaponfromController _self)
  (CallFunction|SetHealthfromController _self)
  (CallFunction|SetSpeedfromController _self))

(event Collision|EventActorBeginOverlap
  (params (OtherActor :type Actor%20Object%20Reference)))

(event EventTick
  (params (DeltaSeconds :type Float%20%28single-precision%29)))

(event EventOnDeath
  (if (== (Math|Random|RandomInteger 10) 0)
    (Game|SpawnActorfromClass "/Game/Character/Pickups/HealthPickupBP.HealthPickupBP_C" (Math|Transform|MakeTransform (Transformation|GetActorLocation) "0, 0, 0" "1,1,1") "Undefined" 0 0)
    (Actor|DestroyActor)))

(fn ConstructionScript)