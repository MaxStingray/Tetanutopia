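; Base AI spawner actor that spawns a limited number of AI of a set class when the player is nearby.
; Tick accumulates a cooldown while spawns remain, then waits for player zero's pawn to be within the activation distance.
; Each spawn uses the spawner's transform, adjusts for collision, decrements the remaining count, resets the cooldown and equips the configured weapon if one is set.
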(event EventBeginPlay)

(event Collision|EventActorBeginOverlap
  (params (OtherActor :type Actor%20Object%20Reference)))

(event EventTick
  (params (DeltaSeconds :type Float%20%28single-precision%29))
  (bind _weapontype (Variables|Default|GetWeaponType))
  (if (> (Variables|Default|GetSpawnAmount) 0)
    (bind _output_get (Variables|Default|SetSpawnCoolDown (+ (Variables|Default|GetSpawnCoolDown) DeltaSeconds)))
    (if (>= _output_get (Variables|Default|GetSpawnDelay))
      (if (<= (Math|Vector|VectorLength (- (Transformation|GetActorLocation (Game|Player|GetPlayerPawn 0)) (Transformation|GetActorLocation))) (Variables|Default|GetActivationDist))
        (bind _returnvalue (Game|SpawnActorfromClass (Variables|Default|GetAIType) (Transformation|GetActorTransform) "AdjustIfPossibleButAlwaysSpawn" 0 0))
        (Variables|Default|SetSpawned true)
        (Variables|Default|SetSpawnAmount (- (Variables|Default|GetSpawnAmount) 1))
        (Variables|Default|SetSpawnCoolDown 0.0)
        (if (and (!= _weapontype 0) (!= _weapontype "/Game/AI/Spawners/DoNotEquipe.DoNotEquipe_C"))
          (Class|MasterAI|EquipWeapon _returnvalue _weapontype))))))

(fn ConstructionScript)