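; Boss enemy Blueprint that starts with 1000 health and handles the end of the fight when it dies.
; On death it optionally spawns a next-level node at its X/Y position and plays a head explosion effect.
; It then explodes and destroys every MasterAIBP actor in the world, calling its own DestroyActor inside that same loop rather than after it completes.
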(event EventBeginPlay
  (Variables|Default|SetmaxHealth 1000)
  (Variables|Default|Sethealth 1000))

(event Collision|EventActorBeginOverlap
  (params (OtherActor :type Actor%20Object%20Reference)))

(event EventTick
  (params (DeltaSeconds :type Float%20%28single-precision%29)))

(event EventOnDeath
  (bind _returnvalue (Transformation|GetActorLocation))
  (if (Variables|Default|GetShouldSpawnNode)
    (Game|SpawnActorfromClass "/Game/GameBP/NextLevelNode.NextLevelNode_C" (Math|Transform|MakeTransform (Math|Vector|MakeVector (.x _returnvalue) (.y _returnvalue) 1e+02) "0, 0, 0" "1,1,1") "AlwaysSpawn" 0 0))
  (Effects|SpawnEmitteratLocation "/Game/Geometry_GT/Particles/Effects/particles/BossHeadEplosion.BossHeadEplosion" (Transformation|GetWorldLocation (Variables|Default|GetCapsuleComponent)))
  (bind _outactors (Actor|GetAllActorsOfClass "/Game/AI/MasterComponents/MasterAIBP.MasterAIBP_C"))
  (for _array_element _outactors
    (Effects|SpawnEmitteratLocation "/Game/Geometry_GT/Particles/Effects/particles/P_Explosion_Kamikaze.P_Explosion_Kamikaze" (Transformation|GetWorldLocation (Variables|/Script/Engine.Actor|GetRootComponent _array_element)))
    (Actor|DestroyActor _array_element)
    (Actor|DestroyActor)))

(fn ConstructionScript)