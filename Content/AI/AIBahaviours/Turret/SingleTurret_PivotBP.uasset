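; Single turret pivot actor that sweeps its yaw back and forth, in the turret AI behaviour set.
; Each Tick adds PivotSpeed to the world yaw and flips its sign when the yaw reaches or passes plus or minus PivotMax.
; The step is not scaled by DeltaSeconds, so sweep speed depends on frame rate, and the limits are centred on world zero rather than the placed rotation.
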(event EventBeginPlay
  (|CallParentFunction))

(event Collision|EventActorBeginOverlap
  (params (OtherActor :type Actor%20Object%20Reference))
  (|CallParentFunction OtherActor) ; This node is disabled and will not be called.\nDrag off pins to build functionality.
)

(event EventTick
  (params (DeltaSeconds :type Float%20%28single-precision%29))
  (bind _returnvalue (Transformation|GetActorRotation))
  (bind _pivotmax (Variables|Default|GetPivotMax))
  (|CallParentFunction DeltaSeconds)
  (if (or (>= (.yaw _returnvalue) _pivotmax) (<= (.yaw _returnvalue) (* _pivotmax -1.0)))
    (Variables|Default|SetPivotSpeed (* (Variables|Default|GetPivotSpeed) -1.0)))
  (Transformation|SetActorRotation (Math|Rotator|MakeRotator 0.0 0.0 (+ (.yaw _returnvalue) (Variables|Default|GetPivotSpeed)))))

(fn ConstructionScript
  (|CallParentFunction))