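; Minion Blueprint for the shield boss fight that shows a shield beam linking it to the boss.
; Each tick it searches for ShieldBossBP actors, aims the beam's end point at the first one's relative location, and hides the beam if none exist.
; On death it spawns a visual explosion, with a one-in-eight roll spawning a small health pack; DestroyActor runs only on that successful roll.
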(event EventBeginPlay
  (|CallParentFunction))

(event Collision|EventActorBeginOverlap
  (params (OtherActor :type Actor%20Object%20Reference))
  (|CallParentFunction OtherActor) ; This node is disabled and will not be called.\nDrag off pins to build functionality.
)

(event EventTick
  (params (DeltaSeconds :type Float%20%28single-precision%29))
  (|CallParentFunction DeltaSeconds)
  (bind _outactors (Actor|GetAllActorsOfClass "/Game/AI/AIBahaviours/ShieldBoss/ShieldBossBP.ShieldBossBP_C"))
  (if (> (Utilities|Array|Length _outactors) 0)
    (Rendering|SetVisibility (Variables|Default|GetShieldBeam) true false)
    (Effects|Components|ParticleSystem|SetVectorParameter (Variables|Default|GetShieldBeam) "Laser_End_Point" (- (Transformation|GetActorLocation (Utilities|Array|Get(acopy) _outactors)) (Transformation|GetActorLocation)))
    (else
      (Rendering|SetVisibility (Variables|Default|GetShieldBeam) false false))))

(event EventOnDeath
  (Game|SpawnActorfromClass "/Game/Character/Explosions/VisualOnly_Explosion.VisualOnly_Explosion_C" (Transformation|GetActorTransform) "Undefined" 0 0)
  (if (== (Math|Random|RandomIntegerinRange 0 7) 0)
    (Game|SpawnActorfromClass "/Game/Character/Pickups/Health/HealthSmallPack.HealthSmallPack_C" (Transformation|GetActorTransform) "Undefined" 0 0)
    (Actor|DestroyActor)))

(fn ConstructionScript
  (|CallParentFunction))