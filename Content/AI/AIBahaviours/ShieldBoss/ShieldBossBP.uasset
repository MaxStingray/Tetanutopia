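; Shield boss enemy with a large health pool that shows its shield while invulnerable.
; Each tick it adds delta time to a shield-down timer in its AI blackboard and syncs the shield's visibility to the invulnerability flag.
; On death it spawns a next-level node at a fixed location, only in the Factory_Content level, then destroys itself.
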(event EventBeginPlay
  (Variables|Default|SetmaxHealth 3000)
  (Variables|Default|Sethealth 3000))

(event Collision|EventActorBeginOverlap
  (params (OtherActor :type Actor%20Object%20Reference)))

(event EventTick
  (params (DeltaSeconds :type Float%20%28single-precision%29))
  (bind _returnvalue (AI|GetBlackboard 0))
  (bind _shielddowntimerkeyname (Variables|Default|GetShieldDownTimerKeyName))
  (bind _sheild (Variables|Default|GetSheild))
  (AI|Components|Blackboard|SetValueasFloat _returnvalue _shielddowntimerkeyname (+ (Class|BlackboardComponent|GetValueasFloat _returnvalue _shielddowntimerkeyname) DeltaSeconds))
  (if (Variables|Default|GetInvulerable)
    (Rendering|SetVisibility _sheild true false)
    (else
      (Rendering|SetVisibility _sheild false false))))

(event EventOnDeath
  (bind _returnvalue (Game|GetCurrentLevelName true))
  (if (Utilities|Enum|Equal(Enum) _returnvalue "Factory_Content")
    (Game|SpawnActorfromClass "/Game/GameBP/NextLevelNode.NextLevelNode_C" (Math|Transform|MakeTransform (Math|Vector|MakeVector -8245.0 -2.506e+04 -855.0) "0, 0, 0" "1,1,1") "AdjustIfPossibleButAlwaysSpawn" 0 0))
  (Actor|DestroyActor))

(fn ConstructionScript)